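; Donut actor whose mesh material glows in a set colour while the first directional light found pitches above zero, likely at night.
; BeginPlay creates a dynamic material instance; Tick looks up the light every frame and starts a timeline that lerps RadioactiveGlow from black to GlowColour.
; A Glow flag prevents restarts and clears on finish, so the timeline repeats; otherwise Tick sets the glow black without stopping the timeline.
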(event EventBeginPlay
  (bind _returnvalue (Rendering|Material|CreateDynamicMaterialInstance (Variables|Default|GetDonut) 0 0 "None" :!class /Script/Engine.PrimitiveComponent))
  (Variables|Default|SetMID _returnvalue))

(event EventTick
  (params (DeltaSeconds :type Float%20%28single-precision%29))
  (bind _glowcolour (Variables|Default|GetGlowColour))
  (bind _outactors (Actor|GetAllActorsOfClass "/Script/Engine.DirectionalLight"))
  (if (> (.Pitch (Math|Rotator|BreakRotator (Transformation|GetActorRotation (Utilities|Array|Get(acopy) _outactors)))) 0.0)
    (if (Math|Boolean|Equal(Boolean) (Variables|Default|GetGlow) false)
      (Variables|Default|SetGlow true)
      (bind _glow (Timeline|Timeline_Glow PlayFromStart)
        (:Update
          (Rendering|Material|SetVectorParameterValue (Variables|Default|GetMID) "RadioactiveGlow" (Math|Color|Lerp(LinearColor) (Utilities|Struct|MakeLinearColor 0.0 0.0 0.0 1.0) (Utilities|Struct|MakeLinearColor (.x _glowcolour) (.y _glowcolour) (.z _glowcolour) 1.0) _glow) :!class /Script/Engine.MaterialInstanceDynamic))
        (:Finished
          (Variables|Default|SetGlow false))))
    (else
      (Variables|Default|SetGlow false)
      (Rendering|Material|SetVectorParameterValue (Variables|Default|GetMID) "RadioactiveGlow" (Utilities|Struct|MakeLinearColor 0.0 0.0 0.0 1.0) :!class /Script/Engine.MaterialInstanceDynamic))))

(fn ConstructionScript)